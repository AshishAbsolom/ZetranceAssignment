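; Interactive microwave prop for archviz, with an animated door, spinning food and a cooking cycle.
; A box overlap by the first-person character enables input, letting E toggle the WB_MicrowaveInterface widget and mouse cursor.
; Door events drive the Opening timeline; MicrowaveStart requires a closed door, then lights the interior while the Cooking timeline plays.
; The construction script applies the food mesh and scale, door angle, spin speed and dynamic material.
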(event OnComponentBeginOverlap(Box)
  (params (OverlappedComponent :type Primitive%20Component%20Object%20Reference) (OtherActor :type Actor%20Object%20Reference) (OtherComp :type Primitive%20Component%20Object%20Reference) (OtherBodyIndex :type Integer) (bFromSweep :type Boolean) (SweepResult :type Hit%20Result%20Structure%20%28by%20ref%29))
  (Utilities|Casting|CastToBP_FirstPersonCharacter OtherActor)
  (Input|EnableInput (Game|GetPlayerController 0)))

(event OnComponentEndOverlap(Box)
  (params (OverlappedComponent :type Primitive%20Component%20Object%20Reference) (OtherActor :type Actor%20Object%20Reference) (OtherComp :type Primitive%20Component%20Object%20Reference) (OtherBodyIndex :type Integer))
  (bind _returnvalue (Game|GetPlayerController 0))
  (Utilities|Casting|CastToBP_FirstPersonCharacter OtherActor)
  (Viewport|RemoveAllWidgets)
  (Input|SetInputModeGameOnly _returnvalue false)
  (Variables|/Script/Engine.PlayerController|SetbShowMouseCursor _returnvalue false))

(event Custom|OpenDoors
  (if (not (Variables|Default|GetIsOpened))
    (bind (_direction _doors) (Timeline|Opening PlayFromStart)
      (:Update
        (Transformation|SetRelativeRotation (Variables|Default|GetSM_Microwave_Door) (Math|Rotator|MakeRotator 0.0 0.0 (* (Variables|Default|GetDoorMaxAngle) _doors)) false false))
      (:Finished
        (Variables|Default|SetIsOpened (Utilities|Select :Index _direction :Forward (Class|KismetSystemLibrary|MakeLiteralBool true) :Backward (Class|KismetSystemLibrary|MakeLiteralBool false)))))))

(event Custom|CloseDoors
  (if (Variables|Default|GetIsOpened)
    (bind (_direction _doors) (Timeline|Opening ReverseFromEnd)
      (:Update
        (Transformation|SetRelativeRotation (Variables|Default|GetSM_Microwave_Door) (Math|Rotator|MakeRotator 0.0 0.0 (* (Variables|Default|GetDoorMaxAngle) _doors)) false false))
      (:Finished
        (Variables|Default|SetIsOpened (Utilities|Select :Index _direction :Forward (Class|KismetSystemLibrary|MakeLiteralBool true) :Backward (Class|KismetSystemLibrary|MakeLiteralBool false)))))))

(event Custom|MicrowaveStart
  (if (Variables|Default|GetIsOpened)
    (Development|PrintText "Close The Door")
    (else
      (Variables|Default|SetIsRunning true)
      (Rendering|Components|Light|SetIntensity (Variables|Default|GetPointLight) 5e+02)
      (Timeline|Cooking Play
        (:Update
          (Variables|/Script/Engine.RotatingMovementComponent|SetRotationRate (Variables|Default|GetRotatingMovement) (Math|Rotator|MakeRotator 0.0 0.0 (Variables|Default|GetSpinningSpeed)))
          (Rendering|Material|CreateDynamicMaterialInstance (Variables|Default|GetSM_Microwave_Main) 1 "/Game/UnrealBucket/Library/ArchViz/Microwave/MI_Microwave.MI_Microwave" "None" :!class /Script/Engine.PrimitiveComponent)
          (Rendering|Material|SetScalarParameterValueonMaterials (Variables|Default|GetSM_Microwave_Main) "Emmisive" 0.0))
        (:Finished
          (Rendering|Components|Light|SetIntensity (Variables|Default|GetPointLight) 0.0))))))

(event Input|KeyboardEvents|E
  (params (Key :type Key%20Structure :default "None"))
  (bind _returnvalue (Game|GetPlayerController 0))
  (:Pressed
    (Utilities|FlowControl|FlipFlop
      (:A
        (bind _returnvalue_2 (UserInterface|CreateWidget "/Game/UnrealBucket/Library/ArchViz/Microwave/WB_MicrowaveInterface.WB_MicrowaveInterface_C"))
        (UserInterface|Viewport|AddtoViewport _returnvalue_2 0)
        (Input|SetInputModeGameandUI _returnvalue _returnvalue_2 "DoNotLock" true false)
        (Variables|/Script/Engine.PlayerController|SetbShowMouseCursor _returnvalue true))
      (:B
        (Viewport|RemoveAllWidgets)
        (Input|SetInputModeGameOnly _returnvalue false)
        (Variables|/Script/Engine.PlayerController|SetbShowMouseCursor _returnvalue false)))))

(fn ConstructionScript
  (bind _staticmeshdinner (Variables|Default|GetStaticMeshDinner))
  ;[1 1 1] Add mesh + set scale
  (Components|StaticMesh|SetStaticMesh _staticmeshdinner (Variables|Default|GetFood))
  (Transformation|SetRelativeScale3D _staticmeshdinner (* (Variables|Default|GetSizeVector) (Variables|Default|GetFoodSize)))
  ;[1 1 1] Door
  (Transformation|SetRelativeRotation (Variables|Default|GetSM_Microwave_Door) (Math|Rotator|MakeRotator 0.0 0.0 (* (Variables|Default|GetDoorMaxAngle) (Variables|Default|GetDoorOpening))) false false)
  (Variables|/Script/Engine.RotatingMovementComponent|SetRotationRate (Variables|Default|GetRotatingMovement) (Math|Rotator|MakeRotator 0.0 0.0 (Variables|Default|GetSpinningSpeed)))
  ;[1 1 1] Create Dynamic Materials Instance
  (Rendering|Material|CreateDynamicMaterialInstance (Variables|Default|GetSM_Microwave_Main) 1 "/Game/UnrealBucket/Library/ArchViz/Microwave/MI_Microwave.MI_Microwave" "None" :!class /Script/Engine.PrimitiveComponent)
  (Rendering|Material|SetScalarParameterValueonMaterials (Variables|Default|GetSM_Microwave_Main) "Emmisive" 0.0))